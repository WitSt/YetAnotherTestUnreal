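; Spawner actor that drops rocks and occasional pickups into the play field at a fixed X line with a random Y.
; BeginPlay starts a looping one-second timer that calls spawnRock.
; Each call usually spawns a Rock, with a one-in-ten chance to instead spawn one of three pickups at random: HPup, WeaponD or WeaponQ.
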(event EventBeginPlay
  (Utilities|Time|SetTimerbyFunctionName 0 "spawnRock" 1.0 true))

(event Collision|EventActorBeginOverlap
  (params (OtherActor :type Actor%20Object%20Reference)))

(event EventTick
  (params (DeltaSeconds :type Float%20%28single-precision%29)))

(fn ConstructionScript)

(fn SpawnRock
  (bind _returnvalue (Math|Random|RandomFloatinRange -5e+02 5e+02))
  (bind _returnvalue_2 (Math|Vector|MakeVector 6e+02 _returnvalue 0.0))
  (bind _returnvalue_3 (Math|Transform|MakeTransform _returnvalue_2))
  (if (== (Math|Random|RandomIntegerinRange 1 10) 1)
    (switch int (Math|Random|RandomIntegerinRange 0 2)
      (:0
        (Game|SpawnActorfromClass "/Game/blueprints/HPup.HPup_C" _returnvalue_3 "Undefined" 0 0))
      (:1
        (Game|SpawnActorfromClass "/Game/blueprints/weaponD.weaponD_C" _returnvalue_3 "Undefined" 0 0))
      (:2
        (Game|SpawnActorfromClass "/Game/blueprints/weaponQ.weaponQ_C" _returnvalue_3 "Undefined" 0 0)))
    (else
      (Game|SpawnActorfromClass "/Game/blueprints/rock.rock_C" _returnvalue_3 "Undefined" 0 0))))