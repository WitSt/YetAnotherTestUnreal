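; Player ship for a rock shooter that slides sideways within fixed Y bounds, creates the HUD and fires bullets and missiles.
; Held fire inputs repeat Shoot and ShootAlt on looping timers, while another timer steadily replenishes missile ammo.
; Shoot spawns single, double or quad bullets by current weapon, reverting to single when pickup ammo runs out.
; Capsule overlaps apply rock damage, health and weapon pickups; low HP activates particles, and zero HP just resets health.
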(event OnComponentBeginOverlap(Capsule)
  (params (OverlappedComponent :type Primitive%20Component%20Object%20Reference) (OtherActor :type Actor%20Object%20Reference) (OtherComp :type Primitive%20Component%20Object%20Reference) (OtherBodyIndex :type Integer) (bFromSweep :type Boolean) (SweepResult :type Hit%20Result%20Structure%20%28by%20ref%29))
  (bind _particlesystem (Variables|Default|GetParticleSystem))
  (bind _asrock (Utilities|Casting|CastTorock OtherActor)
    (:then
      (bind _output_get (Variables|Default|SetshipHP (- (Variables|Default|GetshipHP) (Variables|/Game/blueprints/rock.rock_C|GetrockHPmax _asrock))))
      (Default|Die _asrock)
      (if (<= _output_get 150)
        (Components|Activation|Activate _particlesystem false)
        (if (<= _output_get 0)
          (Development|PrintString "dedzik")
          (Variables|Default|SetshipHP 200)
          (Components|Activation|Deactivate _particlesystem))))
    (:CastFailed
      (bind _ashpup (Utilities|Casting|CastToHPup OtherActor)
        (:then
          (Variables|Default|SetshipHP 200)
          (Components|Activation|Deactivate _particlesystem)
          (Actor|DestroyActor _ashpup))
        (:CastFailed
          (bind _asweapon_d (Utilities|Casting|CastToweaponD OtherActor)
            (:then
              (Variables|Default|SetcurrentWeapon 1)
              (Variables|Default|SetammoMain (Variables|/Game/blueprints/weaponD.weaponD_C|GetammoVal _asweapon_d))
              (Actor|DestroyActor _asweapon_d))
            (:CastFailed
              (bind _asweapon_q (Utilities|Casting|CastToweaponQ OtherActor))
              (Variables|Default|SetcurrentWeapon 2)
              (Variables|Default|SetammoMain (Variables|/Game/blueprints/weaponQ.weaponQ_C|GetammoVal _asweapon_q))
              (Actor|DestroyActor _asweapon_q))))))))

(event EventBeginPlay
  (bind _returnvalue (UserInterface|CreateWidget "/Game/blueprints/HUD.HUD_C" (Game|GetPlayerController 0)))
  (UserInterface|Viewport|AddtoViewport _returnvalue 0)
  (Utilities|Time|SetTimerbyFunctionName 0 "missleRegen" 1e+01 true))

(event Collision|EventActorBeginOverlap
  (params (OtherActor :type Actor%20Object%20Reference)))

(event EventTick
  (params (DeltaSeconds :type Float%20%28single-precision%29))
  (bind _returnvalue (Transformation|GetActorLocation))
  (bind _returnvalue_2 (Input|AxisValues|GetshipMove))
  (bind _shipmovevel (Variables|Default|GetshipMoveVel))
  (bind _returnvalue_3 (Math|Float|Clamp(Float) _returnvalue_2 -1.0))
  (bind _y (Math|Vector|BreakVector _returnvalue))
  (bind _returnvalue_4 (* _returnvalue_3 DeltaSeconds _shipmovevel))
  (if (or (and (< _y 5e+02) (> _returnvalue_4 0.0)) (and (> _y -5e+02) (< _returnvalue_4 0.0)))
    (Transformation|AddActorWorldOffset (Math|Vector|MakeVector 0.0 _returnvalue_4 0.0))))

(event Input|ActionEvents|InputActionshipFire
  (params (Key :type Key%20Structure :default "None"))
  (:Pressed
    (CallFunction|Shoot)
    (bind _returnvalue (Utilities|Time|SetTimerbyFunctionName 0 "shoot" 0.4 true)))
  (:Released
    (Utilities|Time|ClearandInvalidateTimerbyHandle _returnvalue)))

(event Input|ActionEvents|InputActionshipFireAlt
  (params (Key :type Key%20Structure :default "None"))
  (:Pressed
    (CallFunction|ShootAlt)
    (bind _returnvalue (Utilities|Time|SetTimerbyFunctionName 0 "shootAlt" 1.0 true)))
  (:Released
    (Utilities|Time|ClearandInvalidateTimerbyHandle _returnvalue)))

(fn ConstructionScript)

(fn Shoot
  (bind _returnvalue (Transformation|GetActorLocation))
  (bind _y (Math|Vector|BreakVector _returnvalue))
  (if (and (!= (Variables|Default|GetcurrentWeapon) 0) (== (Variables|Default|GetammoMain) 0))
    (Variables|Default|SetcurrentWeapon 0))
  (switch int (Variables|Default|GetcurrentWeapon)
    (:0
      (Game|SpawnActorfromClass "/Game/blueprints/bullet.bullet_C" (Math|Transform|MakeTransform (Math|Vector|MakeVector -3.5e+02 _y 0.0)) "Undefined" 0 0))
    (:1
      (Game|SpawnActorfromClass "/Game/blueprints/bulletD.bulletD_C" (Math|Transform|MakeTransform (Math|Vector|MakeVector -4e+02 (+ _y 5e+01) 0.0)) "Undefined" 0 0)
      (Game|SpawnActorfromClass "/Game/blueprints/bulletD.bulletD_C" (Math|Transform|MakeTransform (Math|Vector|MakeVector -4e+02 (+ _y -5e+01) 0.0)) "Undefined" 0 0)
      (bind _result (Math|Integer|DecrementInt (Variables|Default|GetammoMain))
        (:%20%20
          (Variables|Default|SetammoMain _result))))
    (:2
      (Game|SpawnActorfromClass "/Game/blueprints/bulletQ.bulletQ_C" (Math|Transform|MakeTransform (Math|Vector|MakeVector -4e+02 (+ _y 5e+01) 0.0)) "Undefined" 0 0)
      (Game|SpawnActorfromClass "/Game/blueprints/bulletQ.bulletQ_C" (Math|Transform|MakeTransform (Math|Vector|MakeVector -4e+02 (+ _y -5e+01) 0.0)) "Undefined" 0 0)
      (Game|SpawnActorfromClass "/Game/blueprints/bulletQ.bulletQ_C" (Math|Transform|MakeTransform (Math|Vector|MakeVector -4e+02 (+ _y 75.0) 0.0)) "Undefined" 0 0)
      (Game|SpawnActorfromClass "/Game/blueprints/bulletQ.bulletQ_C" (Math|Transform|MakeTransform (Math|Vector|MakeVector -4e+02 (+ _y -75.0) 0.0)) "Undefined" 0 0)
      (bind _result_2 (Math|Integer|DecrementInt (Variables|Default|GetammoMain))
        (:%20%20
          (Variables|Default|SetammoMain _result_2))))))

(fn MissleRegen
  (Variables|Default|SetammoAlt (+ (Variables|Default|GetammoAlt) 10)))

(fn ShootAlt
  (bind _returnvalue (Transformation|GetActorLocation))
  (bind _y (Math|Vector|BreakVector _returnvalue))
  (if (> (Variables|Default|GetammoAlt) 0)
    (Game|SpawnActorfromClass "/Game/blueprints/missle.missle_C" (Math|Transform|MakeTransform (Math|Vector|MakeVector -4e+02 (+ _y 1e+02) 0.0)) "Undefined" 0 0)
    (Game|SpawnActorfromClass "/Game/blueprints/missle.missle_C" (Math|Transform|MakeTransform (Math|Vector|MakeVector -4e+02 (+ _y -1e+02) 0.0)) "Undefined" 0 0)
    (bind _result (Math|Integer|DecrementInt (Variables|Default|GetammoAlt))
      (:%20%20
        (Variables|Default|SetammoAlt _result)))))