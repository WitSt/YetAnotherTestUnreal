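; Destructible rock actor that moves and spins, and awards points to the Ship when destroyed.
; The construction script randomizes rotation rate, hit points and projectile speed, scaling the rock's size in proportion to its hit points.
; RockHit subtracts damage; at zero or below it adds the rock's max HP to the Ship's Points and calls Die.
; Die spawns an explosion at matching scale and destroys the actor.
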(event Custom|RockHit
  (params (damage :type Integer))
  (bind _output_get (Variables|Default|SetrockHP (- (Variables|Default|GetrockHP) damage)))
  (if (<= _output_get 0)
    (bind _returnvalue (Actor|GetActorOfClass "/Game/blueprints/ship.ship_C"))
    (Variables|/Game/blueprints/ship.ship_C|Setpoints _returnvalue (+ (Variables|/Game/blueprints/ship.ship_C|Getpoints _returnvalue) (Variables|Default|GetrockHPmax)))
    (CallFunction|Die)))

(event EventBeginPlay)

(event Collision|EventActorBeginOverlap
  (params (OtherActor :type Actor%20Object%20Reference)))

(event EventTick
  (params (DeltaSeconds :type Float%20%28single-precision%29)))

(fn ConstructionScript
  (bind _minrot (Variables|Default|GetminRot))
  (bind _maxrot (Variables|Default|GetmaxRot))
  ;[1 1 1] Setting random rotation
  (Variables|/Script/Engine.RotatingMovementComponent|SetRotationRate (Variables|Default|GetRotMov) (Math|Rotator|MakeRotator (Math|Conversions|ToFloat(Integer) (Math|Random|RandomIntegerinRange _minrot _maxrot)) (Math|Conversions|ToFloat(Integer) (Math|Random|RandomIntegerinRange _minrot _maxrot)) (Math|Conversions|ToFloat(Integer) (Math|Random|RandomIntegerinRange _minrot _maxrot))))
  ;[1 1 1] Setting random HP and scaling size
  (bind _output_get (Variables|Default|SetrockHPmax (Math|Random|RandomIntegerinRange (Variables|Default|GetminHP) (Variables|Default|GetmaxHP))))
  (Variables|Default|SetrockHP _output_get)
  (Transformation|SetWorldScale3D (Variables|Default|GetDefaultSceneRoot) (* (Math|Vector|MakeVector 1.0 1.0 1.0) (* _output_get (Variables|Default|GetrockHpSizeRatio))))
  (Variables|Default|SetratioVec (* (Math|Vector|MakeVector 1.0 1.0 1.0) (* _output_get (Variables|Default|GetrockHpSizeRatio))))
  ;[1 1 1] Setting random velocity
  (Variables|/Script/Engine.ProjectileMovementComponent|SetInitialSpeed (Variables|Default|GetProjectileMovement) (Math|Random|RandomFloatinRange (Variables|Default|GetminVel) (Variables|Default|GetmaxVel))))

(fn Die
  (Effects|SpawnEmitteratLocation "/Game/StarterContent/Particles/P_Explosion.P_Explosion" (Transformation|GetActorLocation) "0, 0, 0" (Variables|Default|GetratioVec))
  (Actor|DestroyActor))